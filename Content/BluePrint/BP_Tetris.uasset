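; BP_Tetris runs a Tetris game: board construction, next-piece preview, scoring, levels and auto-restart after game over.
; The construction script builds the instanced-mesh grid from Width and Height; Tick drops and shifts the active BP_Block after collision checks.
; Landed pieces become static mesh components, then line traces check their rows top-down, destroying full ones.
; Box traces find blocks to lower, detect blocked spawns and clear the board.
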(event `RestartGameNewGame`
  (set `self.ScoreGame` 0)
  (`self.GameScore`)
  (set `self.LinesGame` 0)
  ;[0.0625 0.0625 0.0625] Restart Game
  (`self.GameLines`)
  (set `self.LvlGame` 0)
  (`self.GameLvl`)
  (set `self.EndGame?` false)
  (`SceneComponent.SetHiddenInGame` (`self.TextRender_EndGame`) true false)
  (`SceneComponent.SetHiddenInGame` (`self.TextRender_EndGameCounter`) true false)
  (set `self.SpeedLeftRight` 0.07)
  (bind _output_get (set `self.SpeedOneTickGameLv1` (`self.BaseGameSpeed`)))
  (set `self.SpeedDown` _output_get)
  (`KismetSystemLibrary.Delay` 1.0)
  (`self.SpawnBpBlock`))

(event `SpawnBpBlock`
  (bind _ref_bpblock_nextblock (`self.Ref_BpBlock_NextBlock`))
  (bind _ref_bpblock (`self.Ref_BpBlock`)
    (:`then`
      ;[0.07292 0.07292 0.07292] Spawn Block
      (`self.CheckEndGame?`)
      (`self.K2_DestroyActor` _ref_bpblock))
    (:`else`
      _))
  (if (`self.EndGame?`)
    ;[0.1198 0.1198 0.1198] End Game
    (`SceneComponent.SetHiddenInGame` (`self.TextRender_EndGame`) false false)
    (`SceneComponent.SetHiddenInGame` (`self.TextRender_EndGameCounter`) false false)
    (set `self.EndGameCounter` 3)
    (`TextRenderComponent.K2_SetText` (`self.TextRender_EndGameCounter`) (`KismetTextLibrary.Conv_IntToText` (`self.EndGameCounter`)) :!label _label)
    (set `self.EndGameCounter` (- (`self.EndGameCounter`) 1))
    (`KismetSystemLibrary.Delay` 1.0)
    (if (< (`self.EndGameCounter`) 0)
      (`self.EndGameRemoveAllBlock`)
      (`self.RestartGameNewGame`)
      (else
        (goto _label)))
    (else
      (`self.Ref_BpBlock_NextBlock`
        (:`then`
          (bind _output_get (set `self.Ref_BpBlock` (`self.Ref_BpBlock_NextBlock`) :!label _label_2))
          (`self.K2_SetActorLocation` _output_get (`SceneComponent.K2_GetComponentLocation` (`self.ArrowCentraPointSpawnBlock`)) false false)
          (`self.SetActorHiddenInGame` _output_get false)
          (`|ExecutionSequence`
            (:`then_0`
              (bind _returnvalue (`|SpawnActorFromClass` (`|GetArrayItem` (`self.AllBlock`) (`KismetMathLibrary.RandomIntegerInRange` 0 6)) (`KismetMathLibrary.MakeTransform` (`SceneComponent.K2_GetComponentLocation` (`self.Arrow_SpawnNextBlock`))) "Undefined" "OverrideRootScale" null null :!label _label_3))
              (bind _asbp_block (cast `/Game/BluePrint/BP_Block` _returnvalue))
              (bind _output_get_2 (set `self.Ref_BpBlock_NextBlock` _asbp_block))
              (`self.SetActorHiddenInGame` _output_get_2 true)
              (set `self.BlocknumberColor` (`KismetMathLibrary.RandomIntegerInRange` 0 (`KismetArrayLibrary.Array_LastIndex` (`self.AllBlockMaterical`))))
              (`PrimitiveComponent.SetMaterial` (`/Game/BluePrint/BP_Block.AllBlock` _ref_bpblock_nextblock) 0 (`|GetArrayItem` (`self.AllBlockMaterical`) (`self.BlocknumberColor`)))
              (`self.SetActorHiddenInGame` _ref_bpblock_nextblock false))
            (:`then_1`
              (`KismetSystemLibrary.Delay` 0.01)
              (`self.SetActorTickEnabled` true))))
        (:`else`
          (`|ExecutionSequence`
            (:`then_0`
              (goto _label_3))
            (:`then_1`
              (goto _label_2))))))))

(event `EventAddStaticMesh`
  ;[0.2031 0.2031 0.2031] Add Static Mesh-Get Location From Bp_block
  (for _array_element (`/Game/BluePrint/BP_Block.AllBlock` (`self.Ref_BpBlock`))
    (bind _returnvalue (`AddComponent|NODE_AddStaticMeshComponent-0` :`RelativeTransform` (`KismetMathLibrary.MakeTransform` (`SceneComponent.K2_GetComponentLocation` _array_element))))
    (`StaticMeshComponent.SetStaticMesh` _returnvalue (`StaticMeshComponent.StaticMesh` _array_element))
    (`PrimitiveComponent.SetMaterial` _returnvalue 0 (`PrimitiveComponent.GetMaterial` _array_element 0))))

(event `self.ReceiveBeginPlay`
  (`self.RestartGameNewGame`))

(event `BlockSortLocation`
  (bind _detectblocklocationz (`self.DetectBlockLocationZ`))
  (bind (_indexofmaxvalue _maxvalue) (`KismetMathLibrary.MaxOfIntArray` (`self.DetectBlockLocationZ`)))
  ;[0.2083 0.2083 0.2083] Get Location From All Block-Remove Duble Location-And Sort Location
  (`KismetArrayLibrary.Array_Clear` (`self.DetectBlockLocationZ_Sort`))
  (`KismetArrayLibrary.Array_Clear` (`self.DetectBlockLocationZ`))
  ;;[0.08333 0.08333 0.08333] Get all Block -Get Block Location-Remove Duble Location
  (for (_array_element _array_index) (`/Game/BluePrint/BP_Block.AllBlock` (`self.Ref_BpBlock`))
    (if (== _array_index 0)
      (bind (_returnvalue_x _returnvalue_y _returnvalue_z) (`KismetMathLibrary.BreakVector` (`SceneComponent.K2_GetComponentLocation` _array_element)))
      (bind _returnvalue (`KismetMathLibrary.FTrunc` _returnvalue_z))
      (`KismetArrayLibrary.Array_Add` (`self.DetectBlockLocationZ`) _returnvalue :!label _label_4)
      (elif (== (`KismetArrayLibrary.Array_Find` (`self.DetectBlockLocationZ`) _returnvalue) -1)
        (goto _label_4))))
  ;;[0.08854 0.08854 0.08854] Sort Int
  (`KismetArrayLibrary.Array_Add` (`self.DetectBlockLocationZ_Sort`) _maxvalue :!label _label_5)
  (`KismetArrayLibrary.Array_Remove` _detectblocklocationz _indexofmaxvalue)
  (if (`KismetArrayLibrary.Array_IsValidIndex` _detectblocklocationz)
    (goto _label_5)
    (else
      (set `self.DetectBlockGetIndex` -1)
      (`self.DetectBlockFullLine`))))

(event `KeyRight`
  (params (`Press?` :type Boolean))
  (set `self.Right` `Press?`))

(event `KeyLeft`
  (params (`Press?` :type Boolean))
  (set `self.Left` `Press?`))

(event `KeyUp`
  (params (`Press?` :type Boolean))
  (if `Press?`
    (`/Game/BluePrint/BP_Block.BlockRotation` (`self.Ref_BpBlock`))))

(event `KeyDown`
  (params (`Press?` :type Boolean))
  (bind _speedonetickgamelv1 (`self.SpeedOneTickGameLv1`))
  (if `Press?`
    (bind _output_get (set `self.SpeedDown` (/ _speedonetickgamelv1 15.0))) ; 玩家按下的速度
    (set `self.TimeDownNextTick` (- (`self.TimeDownNextTick`) _output_get))
    (else
      (set `self.SpeedDown` _speedonetickgamelv1) ; 正常下落的速度
    )))

(event `self.ReceiveTick`
  (params (DeltaSeconds :type "Float (single-precision)"))
  (bind _returnvalue (`KismetSystemLibrary.GetGameTimeInSeconds`))
  (`|ExecutionSequence`
    (:`then_0`
      (if (>= _returnvalue (`self.TimeDownNextTick`))
        (set `self.TimeDownNextTick` (+ (`self.SpeedDown`) _returnvalue))
        (bind _collision_ (`/Game/BluePrint/BP_Block.DetectCollison` (`self.Ref_BpBlock`) false true false))
        (if _collision_
          (`self.SetActorTickEnabled` false)
          (set `self.ScoreCounter` 0)
          (`self.SetActorHiddenInGame` (`self.Ref_BpBlock`) true)
          (`self.EventAddStaticMesh`)
          (`self.BlockSortLocation`)
          (else
            (`self.NextBlockLocation` 0)))))
    (:`then_1`
      (if (>= _returnvalue (`self.SpeedLeftRightNextTick`))
        (set `self.SpeedLeftRightNextTick` (+ (`self.SpeedLeftRight`) _returnvalue))
        (if (`self.Left`)
          (bind _collision__2 (`/Game/BluePrint/BP_Block.DetectCollison` (`self.Ref_BpBlock`) false false true))
          (if (not _collision__2)
            (`self.NextBlockLocation` 1))
          (elif (`self.Right`)
            (bind _collision__3 (`/Game/BluePrint/BP_Block.DetectCollison` (`self.Ref_BpBlock`) false false false))
            (if (not _collision__3)
              (`self.NextBlockLocation` 2))))))))

(event `DetectBlockFullLine`
  (bind _detectblockgetindex (`self.DetectBlockGetIndex`))
  (bind _scorecounter (`self.ScoreCounter`))
  (bind _returnvalue (`KismetMathLibrary.Conv_IntToDouble` (`|GetArrayItem` (`self.DetectBlockLocationZ_Sort`) (`self.DetectBlockGetIndex`))))
  ;[0.2031 0.2031 0.2031] Detect Block Full Line
  (set `self.DetectBlockGetIndex` (+ _detectblockgetindex 1)) ; loop
  (if (`KismetArrayLibrary.Array_IsValidIndex` (`self.DetectBlockLocationZ_Sort`) _detectblockgetindex)
    (bind (_outhits _returnvalue_2) (`KismetSystemLibrary.LineTraceMultiForObjects` :`Start` (`KismetMathLibrary.MakeVector` (`KismetMathLibrary.Conv_IntToDouble` (* (- (`self.Width`) 1) 100)) 0.0 _returnvalue) :`End` (`KismetMathLibrary.MakeVector` 100.0 0.0 _returnvalue) :`ObjectTypes` (`|MakeArray` "ObjectTypeQuery1" :!type "EObjectTypeQuery Enum") :`bIgnoreSelf` false))
    (if _returnvalue_2
      (if (== (`KismetArrayLibrary.Array_LastIndex` _outhits) (- (`self.Width`) 2))
        (set `self.ScoreCounter` (+ (`self.ScoreCounter`) 1))
        (for _array_element _outhits
          (`ActorComponent.K2_DestroyComponent` (`.HitComponent` (`GameplayStatics.BreakHitResult` _array_element))))
        (`self.AllBlockOneDegreeDown`)
        (else
          (`self.DetectBlockFullLine` :!label _label_6)))
      (else
        (goto _label_6)))
    (else
      ;[0.09896 0.09896 0.09896] Score Game
      (if (not (== (`self.ScoreCounter`) 0))
        (set `self.ScoreGame` (+ (`self.ScoreGame`) (* (`KismetMathLibrary.Clamp` (+ _scorecounter (- _scorecounter 1)) 0 99) (- (`self.Width`) 1))))
        (set `self.LinesGame` (+ (`self.LinesGame`) (`self.ScoreCounter`)))
        (`self.GameLines`)
        (`self.GameScore`)
        ;[0.151 0.151 0.151] Game Lvl--Next Lvl= more game speed
        (set `self.LvlGame` (/ (`self.LinesGame`) 10))
        (if (> (`self.LvlGame`) (`self.LvlGame_0`))
          (set `self.LvlGame_0` (`self.LvlGame`))
          (`self.GameLvl`)
          (set `self.SpeedOneTickGameLv1` (- (`self.BaseGameSpeed`) (* (`KismetMathLibrary.Conv_IntToDouble` (`self.LvlGame`)) 0.03)))
          (set `self.SpeedDown` (`self.SpeedOneTickGameLv1`))))
      (`self.SpawnBpBlock`))))

(event `AllBlockOneDegreeDown`
  (bind (_returnvalue_x _returnvalue_y _returnvalue_z) (`KismetMathLibrary.BreakVector` (`SceneComponent.K2_GetComponentLocation` (`self.ArrowCentraPointSpawnBlock`))))
  ;[0.2552 0.2552 0.2552] All Block One Degree Down
  (`KismetArrayLibrary.Array_Clear` (`self.BlockOneDegreeDown`))
  (set `self.BlockDownCounter` 0)
  (bind (_outhits _returnvalue) (`KismetSystemLibrary.BoxTraceMultiForObjects` :`Start` (`KismetMathLibrary.MakeVector` _returnvalue_x 0.0 _returnvalue_z) :`End` (`KismetMathLibrary.MakeVector` _returnvalue_x 0.0 (`KismetMathLibrary.Conv_IntToDouble` (`|GetArrayItem` (`self.DetectBlockLocationZ_Sort`) (`self.DetectBlockGetIndex`)))) :`HalfSize` (`KismetMathLibrary.MakeVector` (`KismetMathLibrary.Conv_IntToDouble` (/ (* (- (`self.Width`) 2) 100) 2))) :`ObjectTypes` (`|MakeArray` "ObjectTypeQuery1" :!type "EObjectTypeQuery Enum") :`bIgnoreSelf` false))
  (if _returnvalue
    (for _array_element _outhits
      (`KismetArrayLibrary.Array_Add` (`self.BlockOneDegreeDown`) (`.HitComponent` (`GameplayStatics.BreakHitResult` _array_element))))
    (`KismetSystemLibrary.Delay` 0.01 :!label _label_7)
    (bind _output_get (set `self.BlockDownCounter` (+ (`self.BlockDownCounter`) 1)))
    (if (> _output_get 2)
      (`self.DetectBlockFullLine`)
      (else
        (for _array_element_2 (`self.BlockOneDegreeDown`)
          (`SceneComponent.K2_SetWorldLocation` _array_element_2 (- (`SceneComponent.K2_GetComponentLocation` _array_element_2) (0.0 0.0 50.0)) true false))
        (goto _label_7)))
    (else
      (`KismetSystemLibrary.Delay` 0.02)
      (`self.DetectBlockFullLine`))))

(event `CheckEndGame?`
  (bind _returnvalue (`SceneComponent.K2_GetComponentLocation` (`self.ArrowCentraPointSpawnBlock`)))
  ;[0.06771 0.06771 0.06771] Check Game is End??
  (if (== _returnvalue (`SceneComponent.K2_GetComponentLocation` (`/Game/BluePrint/BP_Block.Sm_Center` (`self.Ref_BpBlock`))) :`ErrorTolerance` 20.0)
    (bind (_outhit _returnvalue_2) (`KismetSystemLibrary.BoxTraceSingleForObjects` :`Start` _returnvalue :`End` (+ _returnvalue (0.0 0.0 1.0)) :`HalfSize` (45.0 20.0 45.0) :`ObjectTypes` (`|MakeArray` "ObjectTypeQuery1" :!type "EObjectTypeQuery Enum") :`bIgnoreSelf` false))
    (set `self.EndGame?` _returnvalue_2)))

(event `EndGameRemoveAllBlock`
  (bind (_returnvalue_x _returnvalue_y _returnvalue_z) (`KismetMathLibrary.BreakVector` (`SceneComponent.K2_GetComponentLocation` (`self.ArrowCentraPointSpawnBlock`))))
  (bind _outhits (`KismetSystemLibrary.BoxTraceMultiForObjects` :`Start` (`KismetMathLibrary.MakeVector` _returnvalue_x 0.0 _returnvalue_z) :`End` (`KismetMathLibrary.MakeVector` _returnvalue_x 0.0 100.0) :`HalfSize` (`KismetMathLibrary.MakeVector` (`KismetMathLibrary.Conv_IntToDouble` (/ (* (- (`self.Width`) 2) 100) 2))) :`ObjectTypes` (`|MakeArray` "ObjectTypeQuery1" :!type "EObjectTypeQuery Enum") :`bIgnoreSelf` false))
  (for _array_element _outhits
    (`ActorComponent.K2_DestroyComponent` (`.HitComponent` (`GameplayStatics.BreakHitResult` _array_element)))))

(fn `NextBlockLocation`
  (params (Selection :type Integer))
  (locals (L_Location :type "Vector Structure"))
  (switch `int` Selection
    (:`0`
      (set `local.L_Location` (0.0 0.0 100.0)))
    (:`1`
      (set `local.L_Location` (100.0 0.0 0.0)))
    (:`2`
      (set `local.L_Location` (-100.0 0.0 0.0))))
  (`self.K2_SetActorLocation` (`self.Ref_BpBlock`) (- (`self.K2_GetActorLocation` (`self.Ref_BpBlock`)) (`local.L_Location`)) false false))

(fn `UserConstructionScript`
  (bind _returnvalue (* (- (`self.Height`) 1) 100))
  (bind _returnvalue_2 (`KismetMathLibrary.Conv_IntToDouble` (* (/ (`self.Width`) 2) 100)))
  (bind _returnvalue_3 (`KismetMathLibrary.Conv_IntToDouble` (/ _returnvalue 2)))
  (`SceneComponent.K2_SetRelativeLocation` (`self.ArrowCentraPointSpawnBlock`) (`KismetMathLibrary.MakeVector` _returnvalue_2 0.0 (`KismetMathLibrary.Conv_IntToDouble` _returnvalue)) false false)
  (`SceneComponent.K2_SetRelativeLocation` (`self.Arrow_SpawnNextBlock`) (`KismetMathLibrary.MakeVector` (`KismetMathLibrary.Conv_IntToDouble` (+ (* (`self.Width`) 100) 350)) 0.0 (`KismetMathLibrary.Conv_IntToDouble` (- _returnvalue 100))) false false)
  (`SceneComponent.K2_SetWorldLocation` (`self.TextRender_EndGame`) (`KismetMathLibrary.MakeVector` _returnvalue_2 400.0 _returnvalue_3) false false)
  (`SceneComponent.K2_SetWorldLocation` (`self.TextRender_EndGameCounter`) (`KismetMathLibrary.MakeVector` _returnvalue_2 400.0 (- _returnvalue_3 150.0)) false false)
  (for _index (range (+ (`self.Width`) 1))
    (for _index_2 (range (+ (`self.Height`) 1))
      (`InstancedStaticMeshComponent.AddInstance` (`self.HierarchicalInstancedStaticMesh`) (`KismetMathLibrary.MakeTransform` (`KismetMathLibrary.MakeVector` (`KismetMathLibrary.Conv_IntToDouble` (* _index 100)) (`KismetMathLibrary.SelectFloat` 0.0 -90.0 (or (== _index 0) (== _index (`self.Width`)) (== _index_2 0) (== _index_2 (`self.Height`)))) (`KismetMathLibrary.Conv_IntToDouble` (* _index_2 100))))))))